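; Game state that holds a shared mailbox message log and username list for an HTML-based in-game web UI.
; The server update event appends newline-stripped input to the mailbox, then calls the multicast update, which refreshes each player's WebUI through its pawn's controller and scrolls after a Delay inside the loop.
; A separate multicast event rebuilds non-empty usernames from player pawns and calls each pawn's server list update.
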(event Custom|GS_Server_UpdateMailBoxArray
  (params (input :type String))
  (Utilities|Array|Add (Variables|Default|GetmailboxArray) (Utilities|Struct|MakeStruct_MailBox "" (Utilities|String|Replace input "\\n" " ")))
  (CallFunction|GSMultiCastUpdateClients))

(event Custom|GS_MultiCast_GetNewList
  (Utilities|Array|Clear (Variables|Default|GettotalUsernameList))
  (for _array_element (Variables|Default|GetPlayerArray)
    (bind _asnew_blueprint (Utilities|Casting|CastToNewBlueprint (Variables|/Script/Engine.PlayerState|GetPawnPrivate _array_element)))
    (if (not (Utilities|Enum|Equal(Enum) "" (Variables|/Game/NewBlueprint.NewBlueprint_C|Getusername _asnew_blueprint)))
      (Utilities|Array|Add (Variables|Default|GettotalUsernameList) (Variables|/Game/NewBlueprint.NewBlueprint_C|Getusername _asnew_blueprint))))
  (for _array_element_2 (Variables|Default|GetPlayerArray)
    (bind _asnew_blueprint_2 (Utilities|Casting|CastToNewBlueprint (Variables|/Script/Engine.PlayerState|GetPawnPrivate _array_element_2)))
    (Default|ServerUpdateList _asnew_blueprint_2)))

(event Custom|GS_MultiCast_UpdateClients
  (for _array_element (Variables|Default|GetPlayerArray)
    (bind _asnew_blueprint (Utilities|Casting|CastToNewBlueprint (Variables|/Script/Engine.PlayerState|GetPawnPrivate _array_element)))
    (Default|UE4toHTML-UpdateMailBoxList (Variables|/Game/BP_PlayerController.BP_PlayerController_C|GetWebUI (Default|CastedPlayerController _asnew_blueprint)))
    (Utilities|FlowControl|Delay 1.0)
    (Class|WebInterface|Call (Variables|/Game/WebUI.WebUI_C|GetWebInterface_39 (Variables|/Game/BP_PlayerController.BP_PlayerController_C|GetWebUI (Default|CastedPlayerController _asnew_blueprint))) "ScrollToBottom")))

(fn ConstructionScript)