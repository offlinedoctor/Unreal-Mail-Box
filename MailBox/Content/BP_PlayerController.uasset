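; Player controller that hosts a web-based UI for the local player and sends it the player's identity.
; On BeginPlay the local controller creates the WebUI widget and adds it to the viewport.
; EstablishUserSettings waits briefly, reads username and icon from the pawn, packs them into JSON and passes them to the page's UpdateNamesAndIcons function through the web interface.
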(event Custom|EstablishUserSettings
  (Utilities|FlowControl|Delay 0.2)
  (bind _asnew_blueprint (Utilities|Casting|CastToNewBlueprint (Game|Player|GetPlayerPawn 0)))
  (bind _returnvalue (Class|JsonLibraryHelpers|ConstructObject))
  (bind _returnvalue_2 (Class|JsonLibraryHelpers|JsonObjectSetString _returnvalue "username" (Variables|/Game/NewBlueprint.NewBlueprint_C|Getusername _asnew_blueprint)))
  (bind _returnvalue_3 (Class|JsonLibraryHelpers|JsonObjectSetString _returnvalue_2 "icon" (Variables|/Game/NewBlueprint.NewBlueprint_C|Geticon _asnew_blueprint)))
  (Class|WebInterface|Call (Variables|/Game/WebUI.WebUI_C|GetWebInterface_39 (Variables|Default|GetWebUI)) "UpdateNamesAndIcons" (Class|JsonLibraryHelpers|FromObject _returnvalue_3)))

(event EventBeginPlay
  (if (Pawn|IsLocalPlayerController)
    (bind _returnvalue (UserInterface|CreateWidget "/Game/WebUI.WebUI_C"))
    (bind _output_get (Variables|Default|SetWebUI _returnvalue))
    (UserInterface|Viewport|AddtoViewport _output_get 0)
    (Development|PrintString "Hello")))

(fn ConstructionScript)

(fn OnRepIcon)